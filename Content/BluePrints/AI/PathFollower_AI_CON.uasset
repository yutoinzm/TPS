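; AI controller that walks its AI_Character along a chain of linked path nodes.
; On BeginPlay it caches the controlled pawn and moves it toward the character's DesiredNode.
; Each tick it polls the move status, and whenever that differs from DesiredStatus it advances DesiredNode to its NextNode and issues a new MoveToActor.
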(event EventBeginPlay
  (bind _asai_character (Utilities|Casting|CastToAI_Character (Pawn|GetControlledPawn)))
  (bind _output_get (Variables|Default|SetStoredPown _asai_character))
  (AI|Navigation|MovetoActor (Variables|/Game/BluePrints/AI/AI_Character.AI_Character_C|GetDesiredNode _output_get) 1e+01 true true true 0))

(event EventTick
  (params (DeltaSeconds :type Float%20%28single-precision%29))
  (bind _storedpown (Variables|Default|GetStoredPown))
  (if (Utilities|Enum|NotEqual(Enum) (Class|AIController|GetMoveStatus) (Variables|Default|GetDesiredStatus))
    (bind _output_get (Variables|/Game/BluePrints/AI/AI_Character.AI_Character_C|SetDesiredNode _storedpown (Variables|/Game/BluePrints/AI_Helper/PathNode.PathNode_C|GetNextNode (Variables|/Game/BluePrints/AI/AI_Character.AI_Character_C|GetDesiredNode _storedpown))))
    (AI|Navigation|MovetoActor _output_get 1e+01 true true true 0)))

(fn ConstructionScript)